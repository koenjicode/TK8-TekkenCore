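; Blueprint library for loading and saving the game's Tekken core save data.
; GetTekkenCoreSaveData loads and casts the existing slot, or creates a BP_TekkenCoreSaveData object and saves it immediately before returning it.
; SaveTekkenCoreData writes a given save object to the same slot and returns whether it succeeded.
; The getter returns no object if the cast or initial save fails.
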(fn GetTekkenCoreSaveData
  (bind _returnvalue (SaveGame|DoesSaveGameExist (LocalVariables|GetSaveString)))
  (if _returnvalue
    (bind _returnvalue_2 (SaveGame|LoadGamefromSlot (LocalVariables|GetSaveString)))
    (bind _asbp_tekken_core_save_data (Utilities|Casting|CastToBP_TekkenCoreSaveData _returnvalue_2))
    (return _asbp_tekken_core_save_data)
    (else
      (bind _returnvalue_3 (SaveGame|CreateSaveGameObject "/Game/Mods/TekkenCore/Blueprints/Core/BP_TekkenCoreSaveData.BP_TekkenCoreSaveData_C"))
      (bind _returnvalue_4 (SaveGame|SaveGametoSlot _returnvalue_3 (LocalVariables|GetSaveString)))
      (if _returnvalue_4
        (return _returnvalue_3)
        (else
          (return 0))))))

(fn SaveTekkenCoreData
  (params (SaveGameObject :type Save%20Game%20Object%20Reference))
  (bind _returnvalue (SaveGame|SaveGametoSlot SaveGameObject (LocalVariables|GetSaveString)))
  (return _returnvalue))